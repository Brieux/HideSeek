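; Feedforward neural network Blueprint with mutation, evaluated every Tick on values read from IA.Inputs.
; Neurons live in one flat array, built from Layer sizes with random weights, or copied from Copy and mutated.
; Hidden layers are linear weighted sums; the first output uses sigmoid, the others tanh.
; Mutation re-randomizes weights when a random roll exceeds TauxDeMutation, so higher values mutate less.
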(event EventBeginPlay
  (bind _tab_neuronal (Variables|Default|GetTab%20Neuronal))
  (Utilities|FlowControl|Delay 0.1)
  (if (Utilities|Array|IsEmpty (Variables|Default|GetCopy?))
    (CallFunction|InitLayer (Variables|Default|GetLayer))
    (CallFunction|InitWeight (Variables|Default|GetTab%20Neuronal))
    (CallFunction|RandomWeight)
    (Variables|Default|Setactive? true)
    (else
      (for (_array_element _array_index) (Variables|Default|GetCopy?)
        (Utilities|Array|SetArrayElem _tab_neuronal _array_index _array_element true)
        (bind _neurone_mutated (CallFunction|Mutate _array_element))
        (Utilities|Array|SetArrayElem _tab_neuronal _array_index _neurone_mutated true))
      (Variables|Default|Setactive? true))))

(event EventTick
  (params (DeltaSeconds :type Float%20%28single-precision%29))
  (if (Variables|Default|Getactive?)
    (CallFunction|ImportInput)
    (CallFunction|CalcValuewithWeight)))

(fn ConstructionScript)

(fn InitLayer
  (params (LayerData :type Array%20of%20Integers))
  (for (_array_element _array_index) LayerData
    (for _index (range 0 (- _array_element 1))
      (Utilities|Array|Add (Variables|Default|GetTab%20Neuronal) (Utilities|Struct|MakeNeurone _array_index _index 0.0 0)))))

(fn InitWeight
  (params (Tab%20Neuronal :type Array%20of%20Neurone%20Structures))
  (for (_array_element _array_index) Tab%20Neuronal
    (if (not (== (.x _array_element) 0))
      (Utilities|Array|Resize (LocalVariables|GetWeightTemp) (Utilities|Array|Get(acopy) (Variables|Default|GetLayer) (- (.x _array_element) 1)))
      (Utilities|Array|SetArrayElem (Variables|Default|GetTab%20Neuronal) _array_index (Utilities|Struct|MakeNeurone (.x _array_element) (.y _array_element) 0.0 (LocalVariables|GetWeightTemp))))))

(fn RandomWeight
  (for (_array_element _array_index) (Variables|Default|GetTab%20Neuronal)
    (if (not (== (.x _array_element) 0))
      (for _array_element_2 (.weight (Utilities|Array|Get(acopy) (Variables|Default|GetTab%20Neuronal) _array_index))
        (Utilities|Array|Add (LocalVariables|GetNewTemp) (Math|Random|RandomFloatinRange -1.0 1.0)))
      (Utilities|Array|SetArrayElem (Variables|Default|GetTab%20Neuronal) _array_index (Utilities|Struct|MakeNeurone (.x (Utilities|Array|Get(acopy) (Variables|Default|GetTab%20Neuronal) _array_index)) (.y (Utilities|Array|Get(acopy) (Variables|Default|GetTab%20Neuronal) _array_index)) (.value (Utilities|Array|Get(acopy) (Variables|Default|GetTab%20Neuronal) _array_index)) (LocalVariables|GetNewTemp)))
      (Utilities|Array|Clear (LocalVariables|GetNewTemp)))))

(fn ImportInput
  (bind _tab_neuronal (Variables|Default|GetTab%20Neuronal))
  (for _index (range 0 (- (Utilities|Array|Get(acopy) (Variables|Default|GetLayer)) 1))
    (Utilities|Array|SetArrayElem _tab_neuronal _index (Utilities|Struct|MakeNeurone (.x (Utilities|Array|Get(acopy) _tab_neuronal _index)) (.y (Utilities|Array|Get(acopy) _tab_neuronal _index)) (Utilities|Array|Get(acopy) (Variables|/Game/ThirdPerson/Blueprints/BP_ThirdPersonCharacter.BP_ThirdPersonCharacter_C|GetInputs (Variables|Default|GetIA)) _index) (.weight (Utilities|Array|Get(acopy) _tab_neuronal _index))))))

(fn CalcValuewithWeight
  (bind _tab_neuronal (Variables|Default|GetTab%20Neuronal))
  (for (_array_element _array_index) (Variables|Default|GetTab%20Neuronal)
    (if (not (== (.x _array_element) 0))
      (for (_array_element_2 _array_index_2) (.weight _array_element)
        (bind _neruonetoreturn (CallFunction|GetNeurone (- (.x _array_element) 1) _array_index_2))
        (LocalVariables|SetTempValue (+ (LocalVariables|GetTempValue) (* _array_element_2 (.value _neruonetoreturn)))))
      (if (== (.x _array_element) (- (Utilities|Array|Length (Variables|Default|GetLayer)) 1))
        (if (== (.y _array_element) 0)
          (bind _out (CallFunction|Sigmoid (LocalVariables|GetTempValue)))
          (Utilities|Array|SetArrayElem _tab_neuronal _array_index (Utilities|Struct|MakeNeurone (.x _array_element) (.y _array_element) _out (.weight _array_element)))
          (LocalVariables|SetTempValue 0.0)
          (else
            (bind _out_2 (CallFunction|Hyperbolique (LocalVariables|GetTempValue)))
            (Utilities|Array|SetArrayElem _tab_neuronal _array_index (Utilities|Struct|MakeNeurone (.x _array_element) (.y _array_element) _out_2 (.weight _array_element)))
            (LocalVariables|SetTempValue 0.0)))
        (else
          (Utilities|Array|SetArrayElem _tab_neuronal _array_index (Utilities|Struct|MakeNeurone (.x _array_element) (.y _array_element) (LocalVariables|GetTempValue) (.weight _array_element)))
          (LocalVariables|SetTempValue 0.0))))))

(fn GetNeurone
  (params (X :type Integer) (Y :type Integer))
  (bind (_array_element _array_index) (Utilities|Array|ForEachLoopwithBreak (Variables|Default|GetTab%20Neuronal) :!label _label)
    (:LoopBody
      (if (and (== (.x _array_element) X) (== (.y _array_element) Y))
        (LocalVariables|SetTempIndex _array_index)
        (goto _label Break)))
    (:Completed
      (return (Utilities|Array|Get(acopy) (Variables|Default|GetTab%20Neuronal) (LocalVariables|GetTempIndex))))))

(fn Sigmoid
  (params (In :type Float%20%28double-precision%29))
  (return (/ 1.0 (+ 1.0 (Class|KismetMathLibrary|Exp (* In -1.0))))))

(fn Hyperbolique
  (params (In :type Float%20%28double-precision%29))
  (return (/ (- (Class|KismetMathLibrary|Exp In) (Class|KismetMathLibrary|Exp (* In -1.0))) (+ (Class|KismetMathLibrary|Exp In) (Class|KismetMathLibrary|Exp (* In -1.0))))))

(fn Mutate
  (params (NeuroneToMutate :type Neurone%20Structure%20%28by%20ref%29))
  (for _array_element (.Weight (Utilities|Struct|BreakNeurone NeuroneToMutate))
    (Utilities|Array|Add (LocalVariables|GetMutatedTemp) (Math|Float|SelectFloat (Math|Random|RandomFloatinRange -1.0 1.0) _array_element (> (Math|Random|RandomFloat) (Variables|Default|GetTauxDeMutation)))))
  (bind _structout (Utilities|Struct|SetmembersinNeurone NeuroneToMutate (LocalVariables|GetMutatedTemp)))
  (return _structout))